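; Post-process controller actor that plays impact hits (chromatic aberration, camera shake, radial blur, bloom) and drives lens flare, cyber scan and distance distortion effects.
; Construction creates dynamic material instances as post-process blendables.
; PlayImpactHit sets intensities that Tick decays linearly over each effect's time, while refreshing the other effects' parameters.
; A child-actor TickHelper, destroyed at BeginPlay, appears to support editor preview through EditorTick.
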(event Custom|Play%20Impact%20Hit
  (params (Settings :type F%20Impact%20Effect%20Variables%20Structure))
  (bind (_chromtime _chromintensity _shaketime _shakeintensity _shakespeed _radialblurtime _radialblurintensity _bloomtime _bloomintensity) (Utilities|Struct|BreakF_ImpactEffectVariables Settings))
  (Utilities|FlowControl|Sequence
    (:then_0
      (|ChromHit _chromtime _chromintensity))
    (:then_1
      (|ShakeHit _shaketime _shakeintensity _shakespeed))
    (:then_2
      (|BlurHit _radialblurtime _radialblurintensity))
    (:then_3
      (|BloomHit _bloomtime _bloomintensity))))

(event EventBeginPlay
  (Debug|CleanTickHelper))

(event EventTick
  (params (DeltaSeconds :type Float%20%28single-precision%29))
  (CallFunction|RunEffectFunctions)
  (CallFunction|LerpEffects DeltaSeconds))

(event EventEditorTick
  (params (Delta%20Seconds :type Float%20%28double-precision%29))
  (if (not (Variables|Private|GetInPlay?))
    (CallFunction|LerpEffects Delta%20Seconds)
    (CallFunction|RunEffectFunctions)))

(fn ConstructionScript
  (CallFunction|ApplyMaterialInstances)
  (CallFunction|RunEffectFunctions)
  (Debug|AddTickHelper))

(fn DebugImpactHit
  (CallFunction|PlayImpactHit (Variables|Debug|GetDebugImpactHitSettings)))

(fn ApplyMaterialInstances
  (Utilities|FlowControl|Sequence
    (:then_0
      (bind _returnvalue (Rendering|Material|CreateDynamicMaterialInstance "/VextraVisualTools/Materials/Effects/M_CameraShake.M_CameraShake" "None" "None" :!class /Script/Engine.KismetMaterialLibrary))
      (Variables|Private|Materials|SetCamShakeMaterial _returnvalue))
    (:then_1
      (bind _returnvalue_2 (Rendering|Material|CreateDynamicMaterialInstance "/VextraVisualTools/Materials/Effects/M_RadialBlur.M_RadialBlur" "None" "None" :!class /Script/Engine.KismetMaterialLibrary))
      (Variables|Private|Materials|SetRadBlurMaterial _returnvalue_2))
    (:then_2
      (bind _returnvalue_3 (Rendering|Material|CreateDynamicMaterialInstance "/VextraVisualTools/Materials/Effects/M_AnamorphicLensFlares.M_AnamorphicLensFlares" "None" "None" :!class /Script/Engine.KismetMaterialLibrary))
      (Variables|Private|Materials|SetLensFlareMaterial _returnvalue_3))
    (:then_3
      (bind _returnvalue_4 (Rendering|Material|CreateDynamicMaterialInstance "/VextraVisualTools/Materials/Effects/M_CyberScan.M_CyberScan" "None" "None" :!class /Script/Engine.KismetMaterialLibrary))
      (Variables|Private|Materials|SetCyberScanMaterial _returnvalue_4))
    (:then_4
      (bind _returnvalue_5 (Rendering|Material|CreateDynamicMaterialInstance "/VextraVisualTools/Materials/Effects/M_DistanceDistortion.M_DistanceDistortion" "None" "None" :!class /Script/Engine.KismetMaterialLibrary))
      (Variables|Private|Materials|SetDistanceDistortionMaterial _returnvalue_5))
    (:then_5
      (Utilities|Struct|SetmembersinPostProcessSettings (Variables|/Script/Engine.PostProcessComponent|GetSettings (Variables|Default|GetPostProcess)) (Utilities|Struct|MakeWeightedBlendables (Utilities|Array|MakeArray (Utilities|Struct|MakeWeightedBlendable 1.0 (Variables|Private|Materials|GetCamShakeMaterial)) (Utilities|Struct|MakeWeightedBlendable 1.0 (Variables|Private|Materials|GetRadBlurMaterial)) (Utilities|Struct|MakeWeightedBlendable 1.0 (Variables|Private|Materials|GetLensFlareMaterial)) (Utilities|Struct|MakeWeightedBlendable 1.0 (Variables|Private|Materials|GetCyberScanMaterial)) (Utilities|Struct|MakeWeightedBlendable 1.0 (Variables|Private|Materials|GetDistanceDistortionMaterial))))))))

(fn RunEffectFunctions
  (EffectFunc|AnamorphicLensFlaresFunc (Variables|LensFlare|GetAnamorphic%20Lens%20Flares%20Enable?))
  (EffectFunc|CyberScanFunc (Variables|CyberScan|GetCyber%20Scan%20Enable?))
  (EffectFunc|DistanceDistortionFunc))

(fn CyberScanFunc
  (params (IsEnabled :type Boolean))
  (bind _cyberscanmaterial (Variables|Private|Materials|GetCyberScanMaterial))
  (if IsEnabled
    (Rendering|Material|SetScalarParameterValue _cyberscanmaterial "ScrollPinch" (Variables|CyberScan|GetCyber%20Scan%20Scroll%20Pinch) :!class /Script/Engine.MaterialInstanceDynamic)
    (Rendering|Material|SetScalarParameterValue _cyberscanmaterial "ScanLerp" (Variables|CyberScan|GetCyber%20Scan%20Intensity) :!class /Script/Engine.MaterialInstanceDynamic)
    (Rendering|Material|SetScalarParameterValue _cyberscanmaterial "Speed" (Variables|CyberScan|GetCyber%20Scan%20Speed) :!class /Script/Engine.MaterialInstanceDynamic)
    (Rendering|Material|SetScalarParameterValue _cyberscanmaterial "MonoIntensity" (Variables|CyberScan|GetCyber%20Scan%20Mono%20Intensity) :!class /Script/Engine.MaterialInstanceDynamic)
    (Rendering|Material|SetVectorParameterValue _cyberscanmaterial "MonoColor" (Variables|CyberScan|GetCyber%20Scan%20Mono%20Color) :!class /Script/Engine.MaterialInstanceDynamic)
    (else
      (Rendering|Material|SetScalarParameterValue _cyberscanmaterial "ScanLerp" 0.0 :!class /Script/Engine.MaterialInstanceDynamic)))
  (return))

(fn AnamorphicLensFlaresFunc
  (params (IsEnabled :type Boolean))
  (bind _lensflarematerial (Variables|Private|Materials|GetLensFlareMaterial))
  (if IsEnabled
    (Rendering|Material|SetScalarParameterValue _lensflarematerial "FlareLerp" 1.0 :!class /Script/Engine.MaterialInstanceDynamic)
    (Rendering|Material|SetScalarParameterValue _lensflarematerial "ExposureScale" (Variables|LensFlare|GetAnamorphic%20Lens%20Flares%20Exposure%20Scale) :!class /Script/Engine.MaterialInstanceDynamic)
    (Rendering|Material|SetScalarParameterValue _lensflarematerial "BloomThreshold" (Variables|LensFlare|GetAnamorphic%20Lens%20Flares%20Threshold) :!class /Script/Engine.MaterialInstanceDynamic)
    (Rendering|Material|SetScalarParameterValue _lensflarematerial "BloomAnamorphicIntensity" (Variables|LensFlare|GetAnamorphic%20Lens%20Flares%20Intensity) :!class /Script/Engine.MaterialInstanceDynamic)
    (Rendering|Material|SetScalarParameterValue _lensflarematerial "BloomAnamorphicSteps" (Variables|LensFlare|GetAnamorphic%20Lens%20Flares%20Steps) :!class /Script/Engine.MaterialInstanceDynamic)
    (Rendering|Material|SetScalarParameterValue _lensflarematerial "BloomAnamorphicLength" (Variables|LensFlare|GetAnamorphic%20Lens%20Flares%20Length) :!class /Script/Engine.MaterialInstanceDynamic)
    (Rendering|Material|SetVectorParameterValue _lensflarematerial "BloomAnamorphicTint" (Variables|LensFlare|GetAnamorphic%20Lens%20Flares%20Tint) :!class /Script/Engine.MaterialInstanceDynamic)
    (else
      (Rendering|Material|SetScalarParameterValue _lensflarematerial "FlareLerp" 0.0 :!class /Script/Engine.MaterialInstanceDynamic)))
  (return))

(fn DistanceDistortionFunc
  (bind _distancedistortionmaterial (Variables|Private|Materials|GetDistanceDistortionMaterial))
  (Rendering|Material|SetScalarParameterValue _distancedistortionmaterial "Speed" (Variables|NormalDistortion|GetNormal%20Distort%20Movement%20Speed) :!class /Script/Engine.MaterialInstanceDynamic)
  (Rendering|Material|SetScalarParameterValue _distancedistortionmaterial "Size" (Variables|NormalDistortion|GetNormal%20Distort%20Movement%20Scale) :!class /Script/Engine.MaterialInstanceDynamic)
  (Rendering|Material|SetScalarParameterValue _distancedistortionmaterial "DistortionAmount" (Variables|NormalDistortion|GetNormal%20Distort%20Amount) :!class /Script/Engine.MaterialInstanceDynamic)
  (Rendering|Material|SetScalarParameterValue _distancedistortionmaterial "Distance" (Variables|NormalDistortion|GetNormal%20Distort%20Edge%20Distance) :!class /Script/Engine.MaterialInstanceDynamic)
  (Rendering|Material|SetScalarParameterValue _distancedistortionmaterial "EdgeFading" (Variables|NormalDistortion|GetNormal%20Distort%20Edge%20Fading) :!class /Script/Engine.MaterialInstanceDynamic)
  (Rendering|Material|SetScalarParameterValue _distancedistortionmaterial "AffectedBrightness" (Variables|NormalDistortion|GetNormal%20Distort%20Affected%20Brightness) :!class /Script/Engine.MaterialInstanceDynamic)
  (Rendering|Material|SetScalarParameterValue _distancedistortionmaterial "UnaffectedBrightness" (Variables|NormalDistortion|GetNormal%20Distort%20Unaffected%20Brightness) :!class /Script/Engine.MaterialInstanceDynamic)
  (Rendering|Material|SetTextureParameterValue _distancedistortionmaterial "DistortionNormal" (Variables|NormalDistortion|GetNormal%20Distort%20Texture))
  (return))

(fn SetChromIntensity
  (params (Intensity :type Float%20%28double-precision%29))
  (Utilities|Struct|SetmembersinPostProcessSettings (Variables|/Script/Engine.PostProcessComponent|GetSettings (Variables|Default|GetPostProcess)) (* Intensity 1e+01)))

(fn SetShakeIntensity
  (params (Intensity :type Float%20%28double-precision%29))
  (bind _returnvalue (* Intensity 0.01))
  (Rendering|Material|SetScalarParameterValue (Variables|Private|Materials|GetCamShakeMaterial) "ShakePowerY" _returnvalue :!class /Script/Engine.MaterialInstanceDynamic)
  (Rendering|Material|SetScalarParameterValue (Variables|Private|Materials|GetCamShakeMaterial) "ShakePowerX" _returnvalue :!class /Script/Engine.MaterialInstanceDynamic))

(fn SetBlurIntensity
  (params (Intensity :type Float%20%28double-precision%29))
  (Rendering|Material|SetScalarParameterValue (Variables|Private|Materials|GetRadBlurMaterial) "BlurWidth" (* Intensity 0.1) :!class /Script/Engine.MaterialInstanceDynamic))

(fn SetBloomIntensity
  (params (Intensity :type Float%20%28double-precision%29))
  (Utilities|Struct|SetmembersinPostProcessSettings (Variables|/Script/Engine.PostProcessComponent|GetSettings (Variables|Default|GetPostProcess)) (Math|Float|Clamp(Float) (* Intensity 1e+01) 0.675 1e+05)))

(fn LerpShake
  (params (DeltaTime :type Float%20%28double-precision%29))
  (bind _output_get (Variables|Private|Shake|SetCurrentShakeIntensity (Math|Interpolation|FInterptoConstant (Variables|Private|Shake|GetCurrentShakeIntensity) 0.0 DeltaTime (Variables|Private|Shake|GetCurrentShakeTimeSpeed))))
  (Setters|SetShakeIntensity _output_get))

(fn LerpChrom
  (params (DeltaTime :type Float%20%28double-precision%29))
  (bind _output_get (Variables|Private|Chrom|SetCurrentChromIntensity (Math|Interpolation|FInterptoConstant (Variables|Private|Chrom|GetCurrentChromIntensity) 0.0 DeltaTime (Variables|Private|Chrom|GetCurrentChromSpeed))))
  (Setters|SetChromIntensity _output_get))

(fn CleanTickHelper
  (Variables|Private|SetInPlay? true)
  (Components|DestroyComponent (Variables|Default|GetTickHelper)))

(fn AddTickHelper
  (bind _returnvalue (AddComponent|AddChildActorComponent false))
  (Variables|Default|SetTickHelper _returnvalue))

(fn LerpEffects
  (params (InputPin :type Float%20%28single-precision%29))
  (Lerps|LerpChrom InputPin)
  (Lerps|LerpShake InputPin)
  (CallFunction|LerpBlur InputPin)
  (CallFunction|LerpBloom InputPin))

(fn LerpBlur
  (params (DeltaTime :type Float%20%28double-precision%29))
  (bind _output_get (Variables|Private|Blur|SetCurrentBlurIntensity (Math|Interpolation|FInterptoConstant (Variables|Private|Blur|GetCurrentBlurIntensity) 0.0 DeltaTime (Variables|Private|Blur|GetCurrentBlurSpeed))))
  (Setters|SetBlurIntensity _output_get))

(fn LerpBloom
  (params (DeltaTime :type Float%20%28double-precision%29))
  (bind _output_get (Variables|Private|Bloom|SetCurrentBloomIntensity (Math|Interpolation|FInterptoConstant (Variables|Private|Bloom|GetCurrentBloomIntensity) 0.0 DeltaTime (Variables|Private|Bloom|GetCurrentBloomSpeed))))
  (Setters|SetBloomIntensity _output_get))