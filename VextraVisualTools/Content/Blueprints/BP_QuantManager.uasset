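; Music quantization manager that runs a Quartz clock and relays its beat events to actors in the level.
; StartClock, optionally called on BeginPlay, caches every actor implementing BPI_QuantizationEvents, then creates the 4/4 "Main" clock at the current song BPM.
; OnQuantize receives all clock subdivisions and forwards bar, straight-note and triplet ticks to each cached actor through matching interface messages.
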(event Custom|StartClock
  ;[1 1 1] Clock
  (CallFunction|InitializeQuanitizationActors)
  (bind _returnvalue (Class|QuartzSubsystem|CreateNewClock (WorldSubsystems|GetQuartzSubsystem) "Main" (Utilities|Struct|MakeQuartzClockSettings (Utilities|Struct|MakeQuartzTimeSignature 4 "QuarterNote") false) true))
  (bind _output_get (Variables|Default|SetMainClock _returnvalue))
  (bind _clockhandle (Class|QuartzClockHandle|SetBeatsPerMinute _output_get (Utilities|Struct|MakeQuartzQuantizationBoundary "SixteenthNote" 1.0 "BarRelative") 0 (Variables|Settings|GetCurrentSongBPM)))
  (bind _clockhandle_2 (Class|QuartzClockHandle|SubscribetoAllQuantizationEvents _clockhandle (delegate Custom|OnQuantize)))
  (Class|QuartzClockHandle|ResetTransportQuantized _clockhandle_2)
  (Class|QuartzClockHandle|StartClock _clockhandle_2))

(event Custom|OnQuantize
  (params (ClockName :type Name) (QuantizationType :type EQuartzCommandQuantization%20Enum :default "Bar") (NumBars :type Integer) (Beat :type Integer) (BeatFraction :type Float%20%28single-precision%29))
  ;[1 1 1] Clock
  (for _array_element (Variables|Default|GetQuantActors)
    (switch Utilities|FlowControl|Switch|SwitchonEQuartzCommandQuantization QuantizationType
      (:Bar
        (Class|BPIQuantizationEvents|OnBar(Message) _array_element "NewEnumerator0"))
      (:ThirtySecondNote
        (Class|BPIQuantizationEvents|On32nd(Message) _array_element "NewEnumerator7"))
      (:SixteenthNote
        (Class|BPIQuantizationEvents|On16th(Message) _array_element "NewEnumerator5"))
      (:EighthNote
        (Class|BPIQuantizationEvents|OnEight(Message) _array_element "NewEnumerator3"))
      (:QuarterNote
        (Class|BPIQuantizationEvents|OnQuarter(Message) _array_element "NewEnumerator2"))
      (:HalfNote
        (Class|BPIQuantizationEvents|OnHalfBar(Message) _array_element "NewEnumerator1"))
      (:SixteenthNoteTriplet
        (Class|BPIQuantizationEvents|1/24(Triplet)(Message) _array_element "NewEnumerator10"))
      (:EighthNoteTriplet
        (Class|BPIQuantizationEvents|1/12(Triplet)(Message) _array_element "NewEnumerator4"))
      (:QuarterNoteTriplet
        (Class|BPIQuantizationEvents|1/6(Triplet)(Message) _array_element "NewEnumerator6"))
      (:HalfNoteTriplet
        (Class|BPIQuantizationEvents|1/3(Triplet)(Message) _array_element "NewEnumerator9")))))

(event EventBeginPlay
  (if (Variables|Settings|GetStartClockAtSpawn?)
    (CallFunction|StartClock)))

(event Collision|EventActorBeginOverlap
  (params (OtherActor :type Actor%20Object%20Reference)))

(event EventTick
  (params (DeltaSeconds :type Float%20%28single-precision%29)))

(fn ConstructionScript)

(fn InitializeQuanitizationActors
  (Utilities|Array|Clear (Variables|Default|GetQuantActors))
  (bind _outactors (Actor|GetAllActorswithInterface "/VextraVisualTools/Data/Interfaces/BPI_QuantizationEvents.BPI_QuantizationEvents_C"))
  (Variables|Default|SetQuantActors _outactors))