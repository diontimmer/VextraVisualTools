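; BP_TickHelper is a helper actor, meant to live as a child actor, that drives tick-like updates on its parent.
; Its construction script checks whether the parent actor implements BPI_EditorTick and, if so, starts a fast looping timer by function name.
; Each timer firing calls the parent's EditorTickMessage with world delta seconds, giving a tick from construction time rather than relying on the Tick event.
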(event EventBeginPlay)

(event Collision|EventActorBeginOverlap
  (params (OtherActor :type Actor%20Object%20Reference)))

(event EventTick
  (params (DeltaSeconds :type Float%20%28single-precision%29)))

(fn ConstructionScript
  (if (Utilities|DoesObjectImplementInterface (Actor|GetParentActor) "/VextraVisualTools/Data/Interfaces/BPI_EditorTick.BPI_EditorTick_C")
    (Utilities|Time|SetTimerbyFunctionName 0 "FireEditorTick" 0.01 true)))

(fn FireEditorTick
  (Class|BPIEditorTick|EditorTick(Message) (Actor|GetParentActor) (Utilities|Time|GetWorldDeltaSeconds self)))